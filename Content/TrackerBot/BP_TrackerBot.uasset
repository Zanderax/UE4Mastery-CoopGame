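; BP_TrackerBot is a tracker bot actor, mostly stubbed out in this graph.
; Tick scales the audio component's volume with velocity and re-sets a looping one-second timer every frame for the empty CheckNearbyBots event.
; FindNextPathPoint queries a synchronous navigation path to the player pawn but does nothing with the points.
; Its call and the debug-sphere drawing are disconnected, and BeginPlay is empty.
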(event `FindNextPathPoint`
  (bind _returnvalue (`NavigationSystemV1.FindPathToActorSynchronously` (`self.K2_GetActorLocation`) (`GameplayStatics.GetPlayerPawn` 0) 50.0 null null))
  (for _array_element (`NavigationPath.PathPoints` _returnvalue)
    _))

(event `self.ReceiveBeginPlay`)

(event `self.ReceiveTick`
  (params (DeltaSeconds :type "Float (single-precision)"))
  (`AudioComponent.SetVolumeMultiplier` (`self.AudioComp`) (`KismetMathLibrary.MapRangeClamped` (`KismetMathLibrary.VSize` (`self.GetVelocity`)) 0.0 3000.0 0.5 2.0))
  (`KismetSystemLibrary.K2_SetTimerDelegate` (delegate `CheckNearbyBots`) 1.0 true))

(event `CheckNearbyBots`)

(fn `UserConstructionScript`)