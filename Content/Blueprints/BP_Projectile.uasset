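; BP_Projectile is a grenade that launches forward when spawned and explodes to deal area damage.
; BeginPlay applies a mass-scaled forward force to the Grenade component and starts a one-second fuse timer.
; The fuse, or an earlier hit on a BP_TargetDummy, triggers Explode.
; Explode spawns a particle effect, applies flat damage to every actor overlapping DamageRadius, then destroys the projectile.
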(event `self.ReceiveBeginPlay`
  (bind _grenade (`self.Grenade`))
  (`PrimitiveComponent.AddForce` _grenade (* (`SceneComponent.GetForwardVector` _grenade) (* 500000.0 (`PrimitiveComponent.GetMass` (`self.Grenade`)))) "None" false)
  (`KismetSystemLibrary.K2_SetTimerDelegate` (delegate `Explode`) 1.0))

(event `Explode`
  (bind _grenade (`self.Grenade`))
  (`GameplayStatics.SpawnEmitterAtLocation` "/Game/WeaponEffects/Explosion/P_Explosion.P_Explosion" (`SceneComponent.K2_GetComponentLocation` _grenade) (`SceneComponent.K2_GetComponentRotation` _grenade) (2.0 2.0 2.0))
  (for _array_element (`PrimitiveComponent.GetOverlappingActors` (`self.DamageRadius`) null)
    (`GameplayStatics.ApplyDamage` _array_element 20.0))
  (`self.K2_DestroyActor`))

(event `self.ReceiveTick`
  (params (DeltaSeconds :type "Float (single-precision)")))

(event `self.Grenade.OnComponentHit`
  (params (HitComponent :type "PrimitiveComponent Object Reference") (OtherActor :type "Actor Object Reference") (OtherComp :type "PrimitiveComponent Object Reference") (NormalImpulse :type "Vector Structure") (Hit :type "HitResult Structure (by ref)"))
  (cast `/Game/Blueprints/BP_TargetDummy` OtherActor)
  (`self.Explode`))

(fn `UserConstructionScript`)