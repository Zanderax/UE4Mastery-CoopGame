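; BP_TargetDummy is a damageable target dummy that tracks hit combos and ragdolls when killed.
; Each point-damage hit draws a debug sphere at the impact, increments Combo and adds a new WBP_ComboText widget showing the count.
; Every hit also restarts a short timer that resets the combo when it expires.
; When SHealth reports zero or less, the skeletal mesh switches to physics simulation and the actor is removed after a brief lifespan.
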(event `self.ReceivePointDamage`
  (params (Damage :type "Float (single-precision)") (DamageType :type "DamageType Object Reference") (HitLocation :type "Vector Structure") (HitNormal :type "Vector Structure") (HitComponent :type "PrimitiveComponent Object Reference") (BoneName :type Name) (ShotFromDirection :type "Vector Structure") (InstigatedBy :type "Controller Object Reference") (DamageCauser :type "Actor Object Reference") (HitInfo :type "HitResult Structure (by ref)"))
  (`KismetSystemLibrary.DrawDebugSphere` HitLocation 5.0 12 (struct :`R` 0.968856 :`G` 1.0 :`A` 1.0) 3.0)
  (`/Engine/EditorBlueprintResources/StandardMacros.IncrementInt` (`self.Combo`)
    (:`  `
      (if (> (`self.Combo`) 0)
        (bind _returnvalue (`|CreateWidget` "/Game/UI/WBP_ComboText.WBP_ComboText_C" (`GameplayStatics.GetPlayerController` 0)))
        (set `/Game/UI/WBP_ComboText.Combo` (`self.Combo`) _returnvalue)
        (`UserWidget.AddToViewport` _returnvalue 0)
        (`KismetSystemLibrary.K2_SetTimerDelegate` (delegate `EndCombo`) 0.5)))))

(event `EndCombo`
  (set `self.Combo` 0))

(event `self.SHealth.OnHealthChanged`
  (params (HealthComp :type "SHealthComponent Object Reference") (Health :type "Float (single-precision)") (HealthDelta :type "Float (single-precision)") (DamageType :type "DamageType Object Reference") (InstigatedBy :type "Controller Object Reference") (DamageCauser :type "Actor Object Reference"))
  (if (<= Health 0.0)
    (`PrimitiveComponent.SetSimulatePhysics` (`self.SkeletalMesh`) true)
    (`self.SetLifeSpan` 3.0)))

(fn `UserConstructionScript`)