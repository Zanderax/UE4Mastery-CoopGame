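; Player pawn Blueprint that sets up the locally controlled player's HUD on BeginPlay.
; The reticle widget type comes from a DT_WeaponReticle row named after the weapon class's display name, and a health indicator widget is added alongside it.
; Health changes from the health component draw the delta as debug text at the pawn's location.
; Unconnected leftover nodes print health and create a launcher crosshair.
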(event `self.ReceiveBeginPlay`
  (if (`self.IsLocallyControlled`)
    (`|ExecutionSequence`
      (:`then_0`
        (bind _returnvalue (`|GetDataTableRow` "/Game/DataTables/DT_WeaponReticle.DT_WeaponReticle" (`KismetStringLibrary.Conv_StringToName` (`KismetSystemLibrary.GetClassDisplayName` (`self.WeaponClass`))))
          (:`then`
            (bind _returnvalue_2 (`|CreateWidget` (`.ReticleType_5_CD0022A141C827AF76E0ABA3141CDAC4` (break `/Game/DataTables/S_WeaponReticle` _returnvalue)) (`GameplayStatics.GetPlayerController` 0)))
            (`UserWidget.AddToViewport` _returnvalue_2 0))))
      (:`then_1`
        (bind _returnvalue_3 (`|CreateWidget` "/Game/UI/WBP_HealthIndicator.WBP_HealthIndicator_C"))
        (`UserWidget.AddToViewport` _returnvalue_3 0)))))

(event `self.ReceiveTick`
  (params (DeltaSeconds :type "Float (single-precision)")))

(event `self.SHealth.OnHealthChanged`
  (params (HealthComp :type "SHealthComponent Object Reference") (Health :type "Float (single-precision)") (HealthDelta :type "Float (single-precision)") (DamageType :type "DamageType Object Reference") (InstigatedBy :type "Controller Object Reference") (DamageCauser :type "Actor Object Reference"))
  (`KismetSystemLibrary.DrawDebugString` (`self.K2_GetActorLocation`) (`KismetStringLibrary.Conv_DoubleToString` HealthDelta) null (struct :`R` 1.0 :`G` 1.0 :`B` 1.0 :`A` 1.0) 2.0))

(fn `UserConstructionScript`)